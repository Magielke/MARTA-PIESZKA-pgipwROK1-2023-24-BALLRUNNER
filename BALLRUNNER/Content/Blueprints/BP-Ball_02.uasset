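; Player-controlled rolling ball Blueprint with a spring arm camera rig.
; ForwardBack and LeftRight axis inputs apply torque to the Sphere on X and Y, scaled by ForceMultiply and applied as an acceleration change so mass is ignored.
; A separate function changes the camera view by setting the spring arm's length and relative pitch and yaw, with roll held at zero.
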(event Input|AxisEvents|InputAxisForwardBack
  (params (AxisValue :type Float%20%28single-precision%29))
  ;[0.1188 0.1619 1] Ball Movement by torque
  (Class|PrimitiveComponent|AddTorqueinRadians (Variables|Default|GetSphere) (Math|Vector|MakeVector (* AxisValue (Variables|Default|GetForceMultiply)) 0.0 0.0) "None" true))

(event Input|AxisEvents|InputAxisLeftRight
  (params (AxisValue :type Float%20%28single-precision%29))
  ;[0.1188 0.1619 1] Ball Movement by torque
  (Class|PrimitiveComponent|AddTorqueinRadians (Variables|Default|GetSphere) (Math|Vector|MakeVector 0.0 (* AxisValue (Variables|Default|GetForceMultiply)) 0.0) "None" true))

(fn ConstructionScript)

(fn ChangeCameraView02a
  (params (CameraDistance :type Float%20%28single-precision%29) (CameraRotationY :type Float%20%28single-precision%29) (CameraRotationZ :type Float%20%28single-precision%29))
  (bind _springarm (Variables|Default|GetSpringArm))
  (Variables|/Script/Engine.SpringArmComponent|SetTargetArmLength _springarm CameraDistance)
  (Transformation|SetRelativeRotation _springarm (Math|Rotator|MakeRotator 0.0 CameraRotationY CameraRotationZ) false false))