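; BP_Pickup_02 is a crystal pickup that flies into the player when touched.
; Overlap of its Trigger by the player pawn plays a 2D pickup sound, then after a short delay starts the CrystalTransform timeline.
; The timeline lerps the actor from its current position toward the player's live position, shrinks it and fades its PointLight, then destroys it.
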(event OnComponentBeginOverlap(Trigger)
  (params (OverlappedComponent :type Primitive%20Component%20Object%20Reference) (OtherActor :type Actor%20Object%20Reference) (OtherComp :type Primitive%20Component%20Object%20Reference) (OtherBodyIndex :type Integer) (bFromSweep :type Boolean) (SweepResult :type Hit%20Result%20Structure%20%28by%20ref%29))
  ;[0.401 0.1629 0.1629] Crystal trigger+sound
  (if (== OtherActor (Game|Player|GetPlayerPawn 0))
    (Audio|SpawnSound2D "/Game/Sound_EF/698768__ienba__game-pickup.698768__ienba__game-pickup" 1.0 1.0 0.0 0)
    (Utilities|FlowControl|Delay 0.2)
    ;[0.5677 0.5417 0.2661] Crystaltimeanimation
    (bind (_direction _crystallocation _crystalscale _crystallight) (Timeline|CrystalTransform Play)
      (:Update
        (Transformation|SetActorLocation (Math|Vector|Lerp(Vector) (Transformation|GetActorLocation) (Transformation|GetActorLocation (Game|Player|GetPlayerPawn 0)) _crystallocation) false false)
        (Transformation|SetActorScale3D (Math|Vector|Lerp(Vector) (Transformation|GetActorScale3D) "0, 0, 0" _crystalscale))
        (Rendering|Components|Light|SetIntensity (Variables|Default|GetPointLight) (Math|Float|Lerp 1e+03 0.0 _crystallight)))
      (:Finished
        (Actor|DestroyActor)))))

(fn ConstructionScript)